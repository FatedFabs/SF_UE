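; BP_Boss is a boss actor that tracks its health and death state and drives an on-screen boss HUD.
; On BeginPlay it creates WBP_BossHUD, initializes it with the BP_Boss found through GetActorOfClass, and broadcasts starting health through the EHealthUpadted dispatcher.
; TakeDamage ignores hits once dead, otherwise clamps and rebroadcasts health, and only sets IsDead at zero.
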(event EventBeginPlay
  (bind _returnvalue (UserInterface|CreateWidget "/Game/Blueprints/UI/WBP_BossHUD.WBP_BossHUD_C"))
  (UserInterface|Viewport|AddtoViewport _returnvalue 0)
  (bind _returnvalue_2 (Actor|GetActorOfClass "BP_Boss_C"))
  (Default|Initialize _returnvalue _returnvalue_2)
  (Default|CallEHealthUpadted (Variables|Default|GetCurrentHealth) (Variables|Default|GetMaxHealth)))

(event Collision|EventActorBeginOverlap
  (params (OtherActor :type Actor%20Object%20Reference)))

(event EventTick
  (params (DeltaSeconds :type Float%20%28single-precision%29)))

(fn ConstructionScript)

(fn TakeDamage
  (params (Damage :type Float%20%28double-precision%29))
  (bind _maxhealth (Variables|Default|GetMaxHealth))
  (if (not (Variables|Default|GetIsDead))
    (bind _output_get (Variables|Default|SetCurrentHealth (Math|Float|Clamp(Float) (- (Variables|Default|GetCurrentHealth) Damage) 0.0 _maxhealth)))
    (Default|CallEHealthUpadted _output_get _maxhealth)
    (if (== _output_get 0.0)
      (Variables|Default|SetIsDead true))))