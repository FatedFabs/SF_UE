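; Player ship for a rail shooter, carried along a Track spline while input moves the ship mesh sideways and vertically.
; Tick advances the spline pivot, applies the input offset, then interpolates mesh rotation from pivot movement and input-derived velocity.
; Shoot spawns BP_PlayerBullet at the firing point, and damage updates clamped health through CallEHealthUpdated.
; It creates the HUD, tracks score, and on death disables input and shows the retry screen.
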(event EventBeginPlay
  (bind _returnvalue (UserInterface|CreateWidget "/Game/Blueprints/UI/WBP_HUD.WBP_HUD_C"))
  (UserInterface|Viewport|AddtoViewport _returnvalue 0)
  (Default|Initialize _returnvalue self)
  (Default|CallEHealthUpdated (Variables|Default|GetCurrentHealth) (Variables|Default|GetMaxHealth)))

(event EventTick
  (params (DeltaSeconds :type Float%20%28single-precision%29))
  ;[0.15 0.15 0.15 0.5] Move Ship
  (CallFunction|SnaptoSpline DeltaSeconds)
  (CallFunction|PlaneMove DeltaSeconds)
  (CallFunction|RotateBasedonPositionChange DeltaSeconds)
  (CallFunction|RotateBasedonVelocity DeltaSeconds))

(event Game|Damage|EventAnyDamage
  (params (Damage :type Float%20%28single-precision%29) (DamageType :type Damage%20Type%20Object%20Reference) (InstigatedBy :type Controller%20Object%20Reference) (DamageCauser :type Actor%20Object%20Reference))
  (bind _maxhealth (Variables|Default|GetMaxHealth))
  ;[0.15 0.15 0.15 0.5] Event take damage and death
  (Audio|PlaySound2D "/Game/Sounds/hit-8-bit-01.hit-8-bit-01" 1.0 1.0 0.0 0 0)
  (if (not (Variables|Default|GetIsDead))
    (bind _output_get (Variables|Default|SetCurrentHealth (Math|Float|Clamp(Float) (- (Variables|Default|GetCurrentHealth) Damage) 0.0 _maxhealth)))
    (Default|CallEHealthUpdated _output_get _maxhealth)
    (if (== _output_get 0.0)
      (CallFunction|Death))))

(event Input|ActionEvents|InputActionShoot
  (params (Key :type Key%20Structure))
  (bind _firing_point (Variables|Default|GetFiring%20Point))
  (bind _returnvalue (Transformation|GetWorldTransform _firing_point))
  ;[0.15 0.15 0.15 0.5] Shoot
  (:Pressed
    (Game|SpawnActorfromClass "/Game/Blueprints/BP_PlayerBullet.BP_PlayerBullet_C" (Math|Transform|MakeTransform (.location _returnvalue) (.rotation _returnvalue) "1.000000,1.000000,1.000000") "Undefined" "MultiplyWithRoot" 0 0)
    (Audio|PlaySound2D "/Game/Sounds/146725__leszek_szary__laser.146725__leszek_szary__laser" 1.0 1.0 0.0 0 0)))

(fn ConstructionScript)

(fn SnaptoSpline
  (params (DeltaTime :type Float%20%28double-precision%29))
  (bind _output_get (Variables|Default|SetDistanceTravelled (+ (Variables|Default|GetDistanceTravelled) (* DeltaTime (Variables|Default|GetSpeed)))))
  (bind _pivot (Default|GetPivotatDistance (Variables|Default|GetTrack) _output_get))
  (Transformation|SetActorLocationAndRotation (.location _pivot) (.rotation _pivot)))

(fn PlaneMove
  (params (DeltaTime :type Float%20%28double-precision%29))
  (bind _sm_axionclaymore (Variables|Default|GetSM_AxionClaymore))
  (bind _output_get (LocalVariables|SetMovementSpeed (Math|Vector|MakeVector 0.0 (Input|AxisValues|GetMoveHorizontal) (Input|AxisValues|GetMoveVertical))))
  (bind _output_get_2 (LocalVariables|SetAdjustedOffset (+ (Variables|Default|GetOffset) (* (* _output_get (Variables|Default|GetSpeed)) DeltaTime))))
  (bind _output_get_3 (Variables|Default|SetOffset _output_get_2))
  (Transformation|SetRelativeLocation _sm_axionclaymore (Math|Vector|MakeVector (.x (Variables|/Script/Engine.SceneComponent|GetRelativeLocation _sm_axionclaymore)) (.y _output_get_3) (.z _output_get_3)) false false))

(fn RotateBasedonVelocity
  (params (DeltaTime :type Float%20%28double-precision%29))
  (bind _velocity_vector (CallFunction|GetVelocity))
  (bind _sm_axionclaymore (Variables|Default|GetSM_AxionClaymore))
  (bind (_roll _pitch _yaw) (|VelocityToRotations _velocity_vector))
  (Transformation|SetRelativeRotation _sm_axionclaymore (Math|Interpolation|RInterpTo (Variables|/Script/Engine.SceneComponent|GetRelativeRotation _sm_axionclaymore) (Math|Rotator|MakeRotator _roll _pitch _yaw) DeltaTime 4e+01) false false))

(fn GetVelocity
  (bind _returnvalue (Input|AxisValues|GetMoveHorizontal))
  (bind _returnvalue_2 (Input|AxisValues|GetMoveVertical))
  (bind _returnvalue_3 (Math|Vector2D|Normalize2D (Math|Vector2D|MakeVector2D _returnvalue _returnvalue_2)))
  (return (* (Math|Vector|Normalize (+ (* (Transformation|GetActorRightVector) (.x _returnvalue_3)) (* (Transformation|GetActorUpVector) (.y _returnvalue_3)))) (Variables|Default|GetSpeed))))

(fn RotateBasedonPositionChange
  (params (DeltaTime :type Float%20%28double-precision%29))
  (bind _delta (CallFunction|PivotDelta))
  (bind _sm_axionclaymore (Variables|Default|GetSM_AxionClaymore))
  (bind _relativerotation (Variables|/Script/Engine.SceneComponent|GetRelativeRotation _sm_axionclaymore))
  (Transformation|SetRelativeRotation _sm_axionclaymore (Math|Interpolation|RInterpTo (Variables|/Script/Engine.SceneComponent|GetRelativeRotation _sm_axionclaymore) (Math|Rotator|MakeRotator (+ (.roll _relativerotation) (* (Math|Vector|DotProduct _delta (Transformation|GetActorRightVector)) 45.0)) (+ (.pitch _relativerotation) (* (Math|Vector|DotProduct _delta (Transformation|GetActorUpVector)) 15.0)) (.yaw _relativerotation)) DeltaTime 15.0) false false))

(fn PivotDelta
  (bind _returnvalue (Transformation|GetActorLocation))
  (bind _output_get (LocalVariables|SetCalculatedDelta (- (Variables|Default|GetPastPosition) _returnvalue)))
  (Variables|Default|SetPastPosition _returnvalue)
  (return _output_get))

(fn Death
  (Variables|Default|SetIsDead true)
  (Input|DisableInput (Game|GetPlayerController 0))
  (Rendering|SetVisibility (Variables|Default|GetChildActor1) false true)
  (Audio|PlaySound2D "/Game/Sounds/8-bit-explosion.8-bit-explosion" 1.0 1.0 0.0 0 0)
  (bind _returnvalue (UserInterface|CreateWidget "/Game/Blueprints/UI/WBP_RetryScreen.WBP_RetryScreen_C" (Game|GetPlayerController 0)))
  (UserInterface|Viewport|AddtoViewport _returnvalue 0))

(fn AddScore
  (params (Points :type Integer))
  (Variables|Default|SetScore (+ Points (Variables|Default|GetScore))))