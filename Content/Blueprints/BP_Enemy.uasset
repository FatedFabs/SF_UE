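; BP_Enemy is an enemy that moves along the level's BP_SplineTrack at a set speed.
; On BeginPlay it caches the track and BP_MyPlayer through GetActorOfClass, though the player reference is not used in these graphs.
; While not dead, each Tick calls SnapToSpline, which adds Speed times delta time to DistanceTravelled and sets location and rotation from the track's pivot at that distance.
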(event EventBeginPlay
  (bind _returnvalue (Actor|GetActorOfClass "/Game/Blueprints/BP_SplineTrack.BP_SplineTrack_C"))
  (Variables|Default|SetTrack _returnvalue)
  (bind _returnvalue_2 (Actor|GetActorOfClass "/Game/Blueprints/BP_MyPlayer.BP_MyPlayer_C"))
  (Variables|Default|SetPlayer _returnvalue_2))

(event Collision|EventActorBeginOverlap
  (params (OtherActor :type Actor%20Object%20Reference)))

(event EventTick
  (params (DeltaSeconds :type Float%20%28single-precision%29))
  (if (not (Variables|Default|GetIsDead))
    (CallFunction|SnaptoSpline DeltaSeconds)))

(fn ConstructionScript)

(fn SnaptoSpline
  (params (DeltaTime :type Float%20%28double-precision%29))
  (bind _output_get (Variables|Default|SetDistanceTravelled (+ (Variables|Default|GetDistanceTravelled) (* DeltaTime (Variables|Default|GetSpeed)))))
  (bind _pivot (Default|GetPivotatDistance (Variables|Default|GetTrack) _output_get))
  (Transformation|SetActorLocationAndRotation (.location _pivot) (.rotation _pivot)))